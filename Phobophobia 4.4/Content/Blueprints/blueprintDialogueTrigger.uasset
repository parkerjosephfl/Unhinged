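; Trigger volume Blueprint that plays a one-shot dialogue line when overlapped, queued behind dialogue already playing from other triggers.
; The construction script picks the level's sound array from LvlNum, and DialogueNum selects the line.
; On overlap it scans all dialogue triggers, delays by a playing one's remaining time, then plays at its own location.
; A looping timer counts down DialogueDuration and clears IsPlaying, exposing that state to other triggers.
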(event `UpdateDuration`
  (bind _dialogueduration (`self.dialogueDuration`))
  ;[1 1 1] Updates how much time is left in the playing dialogue
  (`/Engine/EditorBlueprintResources/StandardMacros.CompareFloat` _dialogueduration
    (:`>`
      (set `self.dialogueDuration` (- _dialogueduration 0.1)))
    (:`<`
      (set `self.IsPlaying` false)
      (`KismetSystemLibrary.K2_ClearTimer` null))))

(event `self.ReceiveActorBeginOverlap`
  (params (OtherActor :type "Actor Object Reference"))
  (bind _item (`KismetArrayLibrary.Array_Get` (`self.curLvlDialogue`) (`self.dialogueNum`)))
  ;[1 1 1] When someone enters the dialogue trigger, scan every trigger in the level and check to see if any dialogue is playing. If true, set the time left of the dialogue as a delay
  (`/Engine/EditorBlueprintResources/StandardMacros.DoOnce` false
    (:`Completed`
      (bind _outactors (`GameplayStatics.GetAllActorsOfClass` "blueprintDialogueTrigger_C"))
      (for _array_element _outactors
        (`/Engine/EditorBlueprintResources/StandardMacros.IsValid` _array_element
          (:`Is Valid`
            (bind _asblueprintdialoguetrigger_c (cast `/Game/Blueprints/blueprintDialogueTrigger` _array_element))
            (if (`/Game/Blueprints/blueprintDialogueTrigger.IsPlaying` _asblueprintdialoguetrigger_c)
              (set `self.preDuration` (`/Game/Blueprints/blueprintDialogueTrigger.dialogueDuration` _asblueprintdialoguetrigger_c))))))
      ;[1 1 1] Waits until the previous dialogue is completed, then play the triggered dialogue
      (`KismetSystemLibrary.Delay` (`self.preDuration`))
      (set `self.curDialogue` _item)
      (`GameplayStatics.PlaySoundAtLocation` _item (`self.K2_GetActorLocation`) 1.5)
      (set `self.IsPlaying` true)
      (set `self.dialogueDuration` (`SoundBase.Duration` _item))
      (`KismetSystemLibrary.K2_SetTimer` null "UpdateDuration" 0.1 true))))

(fn `UserConstructionScript`
  (switch `int` (`self.lvlNum`)
    (:`0`
      (set `self.curLvlDialogue` (`self.tutorialDialogue`)))
    (:`1`
      (set `self.curLvlDialogue` (`self.Lvl1Dialogue`)))
    (:`3`
      (set `self.curLvlDialogue` (`self.lvl3Dialogue`)))
    (:`4`
      (set `self.curLvlDialogue` (`self.FinaleDialogue`)))))