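; Torch actor Blueprint with a flame effect, flame audio and a light that follow its IsLit state.
; Tick turns all three on once through a DoOnce when IsLit is true.
; While IsLit is false, Tick resets that gate and runs the shutoff logic every frame, deactivating flame and audio and hiding the light.
; The Destroyed event shares the same shutoff path.
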(event `self.ReceiveDestroyed`
  ;[1 1 1] Deactivate fire particle when the torch is destroyed
  (`ActorComponent.Deactivate` (`self.torchFlame`) :!label _label)
  (`ActorComponent.Deactivate` (`self.audioFlame`))
  (`SceneComponent.SetVisibility` (`self.torchLight`) false false))

(event `self.ReceiveTick`
  (params (DeltaSeconds :type "Float (single-precision)"))
  ;[1 1 1] Sets whether the torch is to be lit or not
  (if (`self.isLit?`)
    (`/Engine/EditorBlueprintResources/StandardMacros.DoOnce` false :!label _label_2
      (:`Completed`
        (`ActorComponent.Activate` (`self.torchFlame`) false)
        (`ActorComponent.Activate` (`self.audioFlame`) false)
        (`SceneComponent.SetVisibility` (`self.torchLight`) true false)))
    (else
      (`|ExecutionSequence`
        (:`then_0`
          (goto _label_2 :!via `Reset`))
        (:`then_1`
          (goto _label))))))

(fn `UserConstructionScript`)