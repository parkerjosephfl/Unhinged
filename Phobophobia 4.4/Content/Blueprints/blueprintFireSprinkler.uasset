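; Fire sprinkler actor that puts out a fire it finds below it.
; While its PutOut flag is set, Tick lowers the FireChecker component by a fixed 20-unit step each frame, without sweeping.
; On overlap with a "fire"-tagged blueprintFire, it stores that actor, destroys FireChecker and sets the fire's own PutOut flag.
; Nothing in this Blueprint sets the sprinkler's PutOut flag.
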(event `self.ReceiveTick`
  (params (DeltaSeconds :type "Float (single-precision)"))
  (bind _firechecker (`self.fireChecker`))
  (if (`self.putOut`)
    (`SceneComponent.SetRelativeLocation` _firechecker (+ (`SceneComponent.RelativeLocation` _firechecker) (0.0 0.0 -20.0)) false)))

(event `self.ReceiveActorBeginOverlap`
  (params (OtherActor :type "Actor Object Reference"))
  (if (`self.ActorHasTag` OtherActor "fire")
    (bind _asblueprintfire_c (cast `/Game/Blueprints/blueprintFire` OtherActor))
    (set `self.fire` _asblueprintfire_c)
    (`ActorComponent.K2_DestroyComponent` (`self.fireChecker`))
    (set `/Game/Blueprints/blueprintFire.putOut` true (`self.fire`))))

(fn `UserConstructionScript`)