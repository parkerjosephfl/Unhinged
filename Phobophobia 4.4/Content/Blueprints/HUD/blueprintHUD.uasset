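; HUD Blueprint that draws a square crosshair, an anxiety readout and an optional journal overlay on the canvas.
; DrawHUD runs a sequence: crosshair, gated journal textures for the current page, then anxiety percentage and page number text.
; ShowPages opens or closes the gate, and draw calls read event values from ShowPages, ShowPageNumber and GetAnxiety.
; The crosshair function's hand-icon branch is hard-coded off.
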(event `self.ReceiveDrawHUD`
  (params (SizeX :type Integer) (SizeY :type Integer))
  (bind _returnvalue (`KismetMathLibrary.Conv_IntToDouble` SizeX))
  (`|ExecutionSequence`
    (:`then_0`
      (`self.drawCrosshair` SizeX SizeY))
    (:`then_1`
      ;[1 1 1] Show Pages if On
      (`/Engine/EditorBlueprintResources/StandardMacros.Gate` true :!label _label
        (:`Exit`
          (`self.DrawTextureSimple` "/Game/Textures/JournalPages/journalCover.journalCover" (- _returnvalue 539.2) 0.0 0.2)
          (`self.DrawTextureSimple` "/Game/Textures/JournalPages/page.page" (- _returnvalue 570.0) 0.0 0.2)
          (`self.DrawTextureSimple` (`KismetArrayLibrary.Array_Get` (stale `self.showPages` pages) (stale `self.showPageNumber` pageNumber)) (- _returnvalue 468.8) 50.0 0.2))))
    (:`then_2`
      (`self.DrawText` (`KismetStringLibrary.Conv_DoubleToString` (* (/ (stale `self.getAnxiety` currentAnxiety) (stale `self.getAnxiety` maxAnxiety)) 100.0)) (struct :`R` 1.0 :`G` 1.0 :`B` 1.0 :`A` 1.0) 20.0 20.0)
      (if (stale `self.showPages` `showPages?`)
        (`self.DrawText` (`KismetStringLibrary.Conv_IntToString` (+ (stale `self.showPageNumber` pageNumber) 1)) (struct :`R` 1.0 :`G` 1.0 :`B` 1.0 :`A` 1.0) 150.0 250.0 null 2.0)))))

(event `self.showPages`
  (params (`showPages?` :type Boolean) (pages :type "Array of Texture Object Reference (by ref)"))
  ;[1 1 1] Show Pages if On
  (if `showPages?`
    (goto _label :!via `Open`)
    (else
      (goto _label :!via `Close`))))

(event `self.showPageNumber`
  (params (pageNumber :type Integer))
  ;[1 1 1] Show Pages if On
)

(event `self.getAnxiety`
  (params (currentAnxiety :type "Float (single-precision)") (maxAnxiety :type "Float (single-precision)")))

(fn `drawCrosshair`
  (params (X :type Integer) (Y :type Integer))
  (bind _returnvalue (`KismetMathLibrary.Conv_IntToDouble` (/ Y 2)))
  (bind _returnvalue_2 (`KismetMathLibrary.Conv_IntToDouble` (/ X 2)))
  (if false
    ;[1 1 1] Draw Hand
    (`self.DrawTextureSimple` "/Game/Textures/HUD/Hand-icon.Hand-icon" (- _returnvalue_2 32.0) (- _returnvalue 32.0) 0.25)
    (else
      ;[1 1 1] Crosshairs
      (`self.DrawRect` (struct :`R` 1.0 :`G` 1.0 :`B` 1.0 :`A` 1.0) _returnvalue_2 _returnvalue 10.0 10.0))))

(fn `UserConstructionScript`)